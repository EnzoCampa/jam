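; Slow enemy AI that roams the navmesh and chases the player while they overlap its detection sphere.
; A self-restarting roam event drives AI MoveTo from a randomly delayed start, attacking when it reaches the player.
; Attacks flash the cone's material for a telegraph, then sphere-trace forward to deal blockable, parryable damage.
; BPCDamageSystem handles health behind a health bar widget; death enables cone physics before destroying the actor.
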(event `self.ReceiveBeginPlay`
  (`|ExecutionSequence`
    (:`then_0`
      ; Start l'ia
      (if (`KismetSystemLibrary.IsValid` (`self.GetController`))
        (`KismetSystemLibrary.Delay` (`KismetMathLibrary.Lerp` 0.1 2.0 (`KismetMathLibrary.RandomFloat`)))
        (`self.roaming Lent`)))
    (:`then_1`
      (bind _returnvalue (`|CreateWidget` "/Game/HUD/W_HealthBar.W_HealthBar_C" null self))
      (`WidgetComponent.SetWidget` (`self.Widget`) _returnvalue))))

(event `Attack`
  (bind _returnvalue (`self.K2_GetActorLocation`))
  (if (not (`/Game/DamageSystem/BPC_DamageSystem.bIsDead` (`self.BPC_DamageSystem`)))
    (`PrimitiveComponent.SetMaterial` (`self.Cone`) 0 "/Game/Ennemies/Materials/Mat_LentColorAttacking.Mat_LentColorAttacking")
    (`KismetSystemLibrary.Delay` 0.5)
    (bind _outhit (`KismetSystemLibrary.SphereTraceSingle` _returnvalue (+ _returnvalue (* (`self.GetActorForwardVector`) 100.0)) 20.0 "TraceTypeQuery3"))
    (`PrimitiveComponent.SetMaterial` (`self.Cone`) 0 "/Game/Ennemies/Materials/Mat_LentColorNormal.Mat_LentColorNormal")
    (if true
      (bind (_bblockinghit _binitialoverlap _time _distance _location _impactpoint _normal _impactnormal _physmat _hitactor) (`GameplayStatics.BreakHitResult` _outhit))
      (bind _asbp_third_person_character (cast `/Game/ThirdPerson/Blueprints/BP_ThirdPersonCharacter` _hitactor))
      (bind _wasdamaged (message `/Game/DamageSystem/BPI_Damagable.TakeDamage` _asbp_third_person_character (make `/Game/DamageSystem/S_DamageInfo` (`self.Damage Dealt`) "NewEnumerator1" false true true) (`/Game/ThirdPerson/Blueprints/BP_ThirdPersonCharacter.bIsBlocking` _asbp_third_person_character) (`KismetSystemLibrary.K2_GetTimerElapsedTimeHandle` (`/Game/ThirdPerson/Blueprints/BP_ThirdPersonCharacter.TImerHandle` _asbp_third_person_character))))
      (if _wasdamaged
        (bind _returnvalue_2 (`GameplayStatics.SpawnEmitterAtLocation` "/Engine/Tutorial/SubEditors/TutorialAssets/TutorialParticleSystem.TutorialParticleSystem" _location))
        (`KismetSystemLibrary.Delay` 0.2)
        (`ActorComponent.K2_DestroyComponent` _returnvalue_2))
      (else
        (`KismetSystemLibrary.PrintString` "Hello")))))

(event `roaming Lent`
  (bind _returnvalue (`self.K2_GetActorLocation`))
  ; Ia move
  (if (not (`/Game/DamageSystem/BPC_DamageSystem.bIsDead` (`self.BPC_DamageSystem`)))
    (if (`self.bIsChasing`)
      (`|AIMoveTo` self (0.0 0.0 0.0) (`self.Other Actor`) 50.0
        (:`OnSuccess`
          (`self.Attack`)
          (`KismetSystemLibrary.Delay` 1.0))
        (:`OnFail`
          _))
      (`self.roaming Lent`)
      (else
        (bind _randomlocation (`NavigationSystemV1.K2_GetRandomLocationInNavigableRadius` _returnvalue 2000.0 null null))
        (if (!= _randomlocation _returnvalue :`ErrorTolerance` 100.0)
          (`|SpawnActorFromClass` "/Game/Ennemies/BP_AI_Destination.BP_AI_Destination_C" (`KismetMathLibrary.MakeTransform` _randomlocation) "AlwaysSpawn" "MultiplyWithRoot" null null)
          (`|AIMoveTo` self _randomlocation null
            (:`OnSuccess`
              _)
            (:`OnFail`
              _))
          (`KismetSystemLibrary.Delay` 1.0)
          (`self.roaming Lent`)
          (else
            (`KismetSystemLibrary.Delay` 0.2)
            (`self.roaming Lent`)))))))

(event `self.Sphere.OnComponentBeginOverlap`
  (params (OverlappedComponent :type "PrimitiveComponent Object Reference") (OtherActor :type "Actor Object Reference") (OtherComp :type "PrimitiveComponent Object Reference") (OtherBodyIndex :type Integer) (bFromSweep :type Boolean) (SweepResult :type "HitResult Structure (by ref)"))
  ; Détection du character
  (if (== OtherActor (`GameplayStatics.GetPlayerCharacter` 0))
    (set `self.Other Actor` OtherActor)
    (set `self.bIsChasing` true)))

(event `self.Sphere.OnComponentEndOverlap`
  (params (OverlappedComponent :type "PrimitiveComponent Object Reference") (OtherActor :type "Actor Object Reference") (OtherComp :type "PrimitiveComponent Object Reference") (OtherBodyIndex :type Integer))
  ; Détection du character
  (if (== (`GameplayStatics.GetPlayerCharacter` 0) OtherActor)
    (set `self.Other Actor` null)
    (set `self.bIsChasing` false)))

(event `Death`
  (bind _cone (`self.Cone`))
  (`PrimitiveComponent.SetSimulatePhysics` _cone true)
  (`PrimitiveComponent.SetCollisionEnabled` _cone "QueryAndPhysics")
  (`ActorComponent.K2_DestroyComponent` (`self.Widget`))
  (`KismetSystemLibrary.Delay` 3.0)
  (`self.K2_DestroyActor`))

(event `Blocked`
  (params (CanBeParried :type Boolean))
  (`KismetSystemLibrary.PrintString` "Blocked"))

(event `DamageResponse`
  (params (DamageResponse :type "/Game/DamageSystem/E_DamageResponse Enum" :default "NewEnumerator0"))
  (`KismetSystemLibrary.PrintString` (`|GetEnumeratorNameAsString` DamageResponse)))

(fn `GetCurrentHealth`
  (returns (Health :type "Float (double-precision)"))
  (return (`/Game/DamageSystem/BPC_DamageSystem.Health` (`self.BPC_DamageSystem`))))

(fn `GetMaxHealth`
  (returns (MaxHealth :type "Float (double-precision)"))
  (return (`/Game/DamageSystem/BPC_DamageSystem.MaxHealth` (`self.BPC_DamageSystem`))))

(fn `Heal`
  (params (Amount :type "Float (double-precision)"))
  (returns (NewHealth :type "Float (double-precision)"))
  (bind _newhealth (`/Game/DamageSystem/BPC_DamageSystem.Heal` (`self.BPC_DamageSystem`) Amount))
  (return _newhealth))

(fn `TakeDamage`
  (params (DamageInfo :type "/Game/DamageSystem/S_DamageInfo Structure") (IsBlocking :type Boolean) (PerfectParryTimer :type "Float (double-precision)"))
  (returns (WasDamaged :type Boolean))
  (bind _damaged (`/Game/DamageSystem/BPC_DamageSystem.TakeDamage` (`self.BPC_DamageSystem`) DamageInfo IsBlocking PerfectParryTimer))
  (return _damaged))

(fn `UserConstructionScript`
  (add `/Game/DamageSystem/BPC_DamageSystem.OnDeath` (`self.BPC_DamageSystem`) (`|CreateDelegate` :!event `Death`))
  (add `/Game/DamageSystem/BPC_DamageSystem.OnBLocked` (`self.BPC_DamageSystem`) (`|CreateDelegate` :!event `Blocked`))
  (add `/Game/DamageSystem/BPC_DamageSystem.DamageResponse` (`self.BPC_DamageSystem`) (`|CreateDelegate` :!event `DamageResponse`)))