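; BP_Ennemie_Normal is a basic AI enemy that roams the navmesh, chases the player when nearby and is destroyed when its health runs out.
; After a random start delay, a self-restarting AIMoveTo loop picks random reachable points, spawning a BP_AI_Destination actor at each.
; Sphere overlaps with the player toggle chasing, which the loop applies on its next pass.
; A TakeDamage event subtracts from Health.
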(event `self.ReceiveBeginPlay`
  ; Start l'ia
  (if (`KismetSystemLibrary.IsValid` (`self.GetController`))
    (`KismetSystemLibrary.Delay` (`KismetMathLibrary.Lerp` 0.1 2.0 (`KismetMathLibrary.RandomFloat`)))
    (`self.roaming Normal`)))

(event `roaming Normal`
  (bind _returnvalue (`self.K2_GetActorLocation`))
  ; Ia move
  (if (`self.bIsChasing`)
    (`|AIMoveTo` self (0.0 0.0 0.0) (`self.Other Actor`) 50.0
      (:`OnSuccess`
        _)
      (:`OnFail`
        _))
    (`self.roaming Normal`)
    (else
      (bind _randomlocation (`NavigationSystemV1.K2_GetRandomLocationInNavigableRadius` _returnvalue 2000.0 null null))
      (if (!= _randomlocation _returnvalue :`ErrorTolerance` 100.0)
        (`|SpawnActorFromClass` "/Game/Ennemies/BP_AI_Destination.BP_AI_Destination_C" (`KismetMathLibrary.MakeTransform` _randomlocation) "AlwaysSpawn" "MultiplyWithRoot" null null)
        (`|AIMoveTo` self _randomlocation null
          (:`OnSuccess`
            _)
          (:`OnFail`
            _))
        (`KismetSystemLibrary.Delay` 1.0)
        (`self.roaming Normal`)
        (else
          (`KismetSystemLibrary.Delay` 0.2)
          (`self.roaming Normal`))))))

(event `self.Sphere.OnComponentBeginOverlap`
  (params (OverlappedComponent :type "PrimitiveComponent Object Reference") (OtherActor :type "Actor Object Reference") (OtherComp :type "PrimitiveComponent Object Reference") (OtherBodyIndex :type Integer) (bFromSweep :type Boolean) (SweepResult :type "HitResult Structure (by ref)"))
  ; Détection du character
  (if (== OtherActor (`GameplayStatics.GetPlayerCharacter` 0))
    (set `self.Other Actor` OtherActor)
    (set `self.bIsChasing` true)))

(event `self.Sphere.OnComponentEndOverlap`
  (params (OverlappedComponent :type "PrimitiveComponent Object Reference") (OtherActor :type "Actor Object Reference") (OtherComp :type "PrimitiveComponent Object Reference") (OtherBodyIndex :type Integer))
  ; Détection du character
  (if (== (`GameplayStatics.GetPlayerCharacter` 0) OtherActor)
    (set `self.Other Actor` null)
    (set `self.bIsChasing` false)))

(event `TakeDamage`
  (params (Damage :type "Float (double-precision)"))
  ; Damage
  (bind _output_get (set `self.Health` (- (`self.Health`) Damage)))
  (if (<= _output_get 0.0)
    (`self.K2_DestroyActor`)))

(fn `UserConstructionScript`)