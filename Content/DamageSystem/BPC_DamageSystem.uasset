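; Damage system component that tracks health, healing and death, announcing results through event dispatchers.
; TakeDamage routes each hit through the CanBeDamaged macro as blocked, full or no damage, based on death, invincibility and blocking.
; Blocks broadcast parry eligibility, negating damage within a half-second TimerBlock window and halving it afterward.
; Applied damage triggers OnDeath at zero health, otherwise DamageResponse when interruptible or force-interrupted.
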(fn `Heal`
  (params (Amount :type "Float (double-precision)"))
  (returns (NewHealth :type "Float (double-precision)"))
  (if (not (`self.bIsDead`))
    (bind _output_get (set `self.Health` (`KismetMathLibrary.FClamp` (+ Amount (`self.Health`)) 0.0 (`self.MaxHealth`))))
    (return _output_get)))

(fn `TakeDamage`
  (params (DamageInfo :type "/Game/DamageSystem/S_DamageInfo Structure") (bIsBlocking :type Boolean) (TimerBlock :type "Float (double-precision)"))
  (returns (Damaged :type Boolean))
  (bind (_amount _damageresponse _membeshoulddamageinvincible _canbeblock _canbeparry _shouldforceinterrupt) (break `/Game/DamageSystem/S_DamageInfo` DamageInfo))
  (`self.CanBeDamaged` _membeshoulddamageinvincible _canbeblock bIsBlocking
    (:`BlockDamage`
      (`self.OnBLocked` _canbeparry)
      (if (<= TimerBlock 0.5)
        (return false)
        (else
          (set `self.Health` (- (`self.Health`) (/ _amount 2.0))))))
    (:`DoDamage`
      (bind _output_get (set `self.Health` (- (`self.Health`) _amount))))
    (:`NoDamage`
      (return false)))
  (if (<= _output_get 0.0)
    (set `self.bIsDead` true)
    (`self.OnDeath`)
    (return true)
    (elif (or (`self.bIsInterruptible`) _shouldforceinterrupt)
      (`self.DamageResponse` _damageresponse)
      (return true))))